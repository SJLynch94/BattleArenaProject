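; BP_PowerupQuadDamage is a powerup Blueprint whose name indicates quad damage, though no damage logic appears in its graphs.
; On activation it stores the target actor and casts it to HeroCharacter, but applies no effect.
; On expiry, if that actor is valid, it sets MaxWalkSpeed to half the current max speed and plays a powerdown sound at player 0's pawn.
; It then calls the parent expiry logic.
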(event `self.OnActivated`
  (params (ActivateFor :type "Actor Object Reference"))
  (set `self.ActivatedFor` ActivateFor)
  (bind _ashero_character (cast `HeroCharacter` ActivateFor))
  (`/Engine/EditorBlueprintResources/StandardMacros.IsValid` _ashero_character))

(event `self.OnExpired`
  (bind _activatedfor (`self.ActivatedFor`))
  (bind _returnvalue (`self.GetComponentByClass` _activatedfor "/Script/Engine.CharacterMovementComponent"))
  (`/Engine/EditorBlueprintResources/StandardMacros.IsValid` _activatedfor
    (:`Is Valid`
      (set `CharacterMovementComponent.MaxWalkSpeed` (/ (`MovementComponent.GetMaxSpeed` _returnvalue) 2.0) _returnvalue)
      (`GameplayStatics.PlaySoundAtLocation` "/Game/Powerups/powerdown_01_Cue.powerdown_01_Cue" (`self.K2_GetActorLocation` (`GameplayStatics.GetPlayerPawn` 0)) (struct) 1.0 1.0 0.0 null null null))
    (:`Is Not Valid`
      _))
  (`parent.OnExpired`))

(fn `UserConstructionScript`)