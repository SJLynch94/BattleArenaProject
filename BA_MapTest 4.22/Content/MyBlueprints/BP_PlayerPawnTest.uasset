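; Test player character with rifle and grenade launcher selection, grenade throwing, sprint, reload, pause menu, god mode and map restart.
; Weapon keys spawn a new weapon on every press, attach it to WeaponSocket and toggle mesh visibility.
; Grenades launch with a suggested arc velocity using the muzzle's forward direction.
; BeginPlay creates HUD widgets, Tick maps movement speed to crosshair spread, and health changes display floating damage text.
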(event `self.ReceiveBeginPlay`
  (`|ExecutionSequence`
    (:`then_0`
      (bind _returnvalue (`|CreateWidget` "/Game/MyHUD/DynamicCrossHair.WBCrosshair_C"))
      (bind _output_get (set `self.CrosshairRef` _returnvalue))
      (`UserWidget.AddToViewport` _output_get 0))
    (:`then_1`
      (bind _returnvalue_2 (`|CreateWidget` "/Game/MyHUD/WBP_HealthIndicator.WBP_HealthIndicator_C"))
      (`UserWidget.AddToViewport` _returnvalue_2 0))
    (:`then_2`
      (bind _returnvalue_3 (`|CreateWidget` "/Game/MyHUD/WBP_MyHUD.WBP_MyHUD_C"))
      (`UserWidget.AddToViewport` _returnvalue_3 0))))

(event `InputAction|SelectGLauncher`
  (params (Key :type "Key Structure"))
  (:`Pressed`
    (bind _returnvalue (`|SpawnActorFromClass` "/Game/MyBlueprints/BP_HeroGLauncher.BP_HeroGLauncher_C" (`KismetMathLibrary.MakeTransform` (0.0 0.0 0.0)) "AlwaysSpawn" "OverrideRootScale" self null))
    (bind _output_get (set `self.GLauncherRef` _returnvalue))
    (bind _output_get_2 (set `self.CurrentWeapon` _output_get))
    (`self.K2_AttachToComponent` _output_get_2 (`self.Mesh`) "WeaponSocket" "SnapToTarget" "SnapToTarget" "SnapToTarget" true)
    (`SceneComponent.SetVisibility` (`HeroWeapon.MeshComp` (`self.GLauncherRef`)) true false)
    (`SceneComponent.SetVisibility` (`HeroWeapon.MeshComp` (`self.RifleRef`)) false false)
    (set `self.bIsRifle` false)))

(event `InputAction|SelectRifle`
  (params (Key :type "Key Structure"))
  (:`Pressed`
    (bind _returnvalue (`|SpawnActorFromClass` "/Game/MyBlueprints/BP_HeroWeapon.BP_HeroWeapon_C" (`KismetMathLibrary.MakeTransform` (0.0 0.0 0.0)) "AlwaysSpawn" "OverrideRootScale" self null))
    (bind _output_get (set `self.RifleRef` _returnvalue))
    (bind _output_get_2 (set `self.CurrentWeapon` _output_get))
    (`self.K2_AttachToComponent` _output_get_2 (`self.Mesh`) "WeaponSocket" "SnapToTarget" "SnapToTarget" "SnapToTarget" true)
    (`SceneComponent.SetVisibility` (`HeroWeapon.MeshComp` (`self.GLauncherRef`)) false false)
    (`SceneComponent.SetVisibility` (`HeroWeapon.MeshComp` (`self.RifleRef`)) true false)
    (set `self.bIsRifle` true)))

(event `self.HealthComp.OnHealthChanged`
  (params (HealthComp :type "HealthComponent Object Reference") (Health :type "Float (single-precision)") (HealthDelta :type "Float (single-precision)") (DamageType :type "DamageType Object Reference") (InstigatedBy :type "Controller Object Reference") (DamageCauser :type "Actor Object Reference"))
  (bind _returnvalue (`self.K2_GetActorLocation`))
  (bind _returnvalue_2 (`KismetTextLibrary.Conv_DoubleToText` HealthDelta "HalfToEven" false true 1 324 0 0))
  (`KismetSystemLibrary.DrawDebugString` _returnvalue (`KismetTextLibrary.Conv_TextToString` _returnvalue_2) null (struct :`R` 1.0 :`G` 0.651406 :`A` 1.0) 0.75)
  (message `/Game/UI/ShowDamageText.ShowDamageText` (`PlayerController.GetHUD` (`GameplayStatics.GetPlayerController` 0)) true (`KismetTextLibrary.Conv_TextToString` _returnvalue_2) _returnvalue))

(event `InputAction|GodMode`
  (params (Key :type "Key Structure"))
  (bind _returnvalue (`self.K2_GetActorLocation`))
  (:`Pressed`
    (if (`self.bIsGodMode`)
      (set `self.bIsGodMode` false)
      (set `self.bCanBeDamaged` true)
      (`KismetSystemLibrary.PrintString` "God Mode OFF")
      (`GameplayStatics.PlaySoundAtLocation` "/Game/Powerups/powerdown_01_Cue.powerdown_01_Cue" _returnvalue (struct) 1.0 1.0 0.0 null null null)
      (else
        (set `self.bIsGodMode` true)
        (set `self.bCanBeDamaged` false)
        (`KismetSystemLibrary.PrintString` "God Mode ON")
        (`GameplayStatics.PlaySoundAtLocation` "/Game/MyBlueprints/Sounds/GODLIKE__Unreal_Tournament_Sound_Cue.GODLIKE__Unreal_Tournament_Sound_Cue" _returnvalue (struct) 1.0 1.0 0.0 null null null)))))

(event `InputAction|RestartMap`
  (params (Key :type "Key Structure"))
  (:`Pressed`
    (`GameplayStatics.OpenLevel` "p_Map")))

(event `InputAction|Grenade`
  (params (Key :type "Key Structure"))
  (bind _currentweapon (`self.CurrentWeapon`))
  (bind _returnvalue (`self.K2_GetActorLocation` _currentweapon))
  (bind _returnvalue_2 (`SceneComponent.GetSocketRotation` (`HeroWeapon.MeshComp` _currentweapon) (`HeroWeapon.MuzzleSocketName` _currentweapon)))
  (:`Pressed`
    (bind _returnvalue_3 (`|SpawnActorFromClass` "/Game/MyBlueprints/Grenade/BP_GrenadeTest.BP_GrenadeTest_C" (`KismetMathLibrary.MakeTransform` _returnvalue _returnvalue_2) "Undefined" "OverrideRootScale" self null))
    (bind _outlaunchvelocity (`GameplayStatics.SuggestProjectileVelocity_CustomArc` _returnvalue (* (`KismetMathLibrary.GetForwardVector` _returnvalue_2) (`self.ThrowingMultiplier`))))
    (`PrimitiveComponent.SetPhysicsLinearVelocity` (`/Game/MyBlueprints/Grenade/BP_GrenadeTest.StaticMesh` _returnvalue_3) _outlaunchvelocity false "None")))

(event `InputAction|Reload`
  (params (Key :type "Key Structure"))
  (:`Pressed`
    (`self.Reload`)))

(event `InputAction|Pause`
  (params (Key :type "Key Structure"))
  (:`Pressed`
    (`self.PauseGame`)))

(event `InputAction|Sprint`
  (params (Key :type "Key Structure"))
  (bind _charactermovement (`self.CharacterMovement`))
  (bind _charactermovement_2 (`self.CharacterMovement`))
  (:`Pressed`
    (set `self.bIsSprinting` true)
    (set `CharacterMovementComponent.MaxWalkSpeed` (* (`MovementComponent.GetMaxSpeed` _charactermovement) 1.5) _charactermovement))
  (:`Released`
    (set `self.bIsSprinting` false)
    (set `CharacterMovementComponent.MaxWalkSpeed` (/ (`MovementComponent.GetMaxSpeed` _charactermovement_2) 1.5) _charactermovement_2)))

(event `self.ReceiveTick`
  (params (DeltaSeconds :type "Float (single-precision)"))
  (`self.UpdateCrosshair`))

(fn `PauseGame`
  (`GameplayStatics.SetGamePaused` true)
  (`/Engine/EditorBlueprintResources/StandardMacros.IsValid` (`self.PauseMenu`)
    (:`Is Valid`
      _)
    (:`Is Not Valid`
      (bind _returnvalue (`|CreateWidget` "/Game/UI/PauseMenu/WBP_PauseMenu.WBP_PauseMenu_C" (`GameplayStatics.GetPlayerController` 0)))
      (set `self.PauseMenu` _returnvalue)))
  (`UserWidget.AddToViewport` (`self.PauseMenu`) 0)
  (`WidgetBlueprintLibrary.SetInputMode_UIOnlyEx` (`GameplayStatics.GetPlayerController` 0) (`self.PauseMenu`))
  (set `PlayerController.bShowMouseCursor` true (`GameplayStatics.GetPlayerController` 0)))

(fn `UnpauseGame`
  (bind _returnvalue (`GameplayStatics.GetPlayerController` 0))
  (`GameplayStatics.SetGamePaused` false)
  (`WidgetLayoutLibrary.RemoveAllWidgets`)
  (`WidgetBlueprintLibrary.SetInputMode_GameOnly` _returnvalue)
  (set `PlayerController.bShowMouseCursor` false _returnvalue)
  (`self.UpdateCrosshair`))

(fn `UpdateCrosshair`
  (set `/Game/MyHUD/DynamicCrossHair.crosshair_spread` (`KismetMathLibrary.MapRangeClamped` (`KismetMathLibrary.VSize` (`self.GetVelocity`)) 0.0 1000.0 10.0 100.0) (`self.CrosshairRef`)))

(fn `UserConstructionScript`)