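; BP_GLProjectile is a timed explosive projectile that detonates a set delay after it spawns.
; BeginPlay waits ExplodeDelay, then calls the Explode event; the graph has no impact trigger.
; Explode spawns the explosion particles, applies radial damage credited to the instigator's controller, fires a RadialForce impulse to push nearby objects, plays the sound and destroys the actor.
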(event `self.ReceiveBeginPlay`
  ;[1 1 1] Begin play starts the delay of which the projectile will call Explode, when Explode is called spawn the particle of explosion and apply radial damage with the variables set, following that then play sound at the location of the projectile to be ExplosionSound_Cue, after that we then fire the impulse to then cause the effected actor to be moved by the projectile explosion and then destroy actor so it is no longer on the world.
  (`KismetSystemLibrary.Delay` (`self.ExplodeDelay`))
  (`self.Explode`))

(event `Explode`
  (bind _returnvalue (`self.K2_GetActorLocation`))
  ;[1 1 1] Begin play starts the delay of which the projectile will call Explode, when Explode is called spawn the particle of explosion and apply radial damage with the variables set, following that then play sound at the location of the projectile to be ExplosionSound_Cue, after that we then fire the impulse to then cause the effected actor to be moved by the projectile explosion and then destroy actor so it is no longer on the world.
  (`GameplayStatics.SpawnEmitterAtLocation` "/Game/WeaponEffects/Explosion/P_Explosion.P_Explosion" _returnvalue)
  (`GameplayStatics.ApplyRadialDamage` :`BaseDamage` (`self.GLDamage`) :`Origin` _returnvalue :`DamageRadius` (`self.DamageRadius`) :`DamageCauser` self :`InstigatedByController` (`self.GetInstigatorController`))
  (`RadialForceComponent.FireImpulse` (`self.RadialForce`))
  (`GameplayStatics.PlaySoundAtLocation` "/Game/ExplosiveBarrel/ExplosionSound/ExplosionSound_Cue.ExplosionSound_Cue" (`self.K2_GetActorLocation`) (struct) 1.0 1.0 0.0 null null null)
  (`self.K2_DestroyActor`))

(fn `UserConstructionScript`)