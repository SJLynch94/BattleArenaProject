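; BP_MyGrenade is a grenade actor that explodes on its own shortly after it spawns.
; BeginPlay waits a brief fixed delay, then calls the Detonate event.
; Detonate spawns a particle emitter, applies radial damage credited to the instigator's controller, fires a RadialForce impulse and plays an explosion sound at the actor's location.
; The graph does not destroy the actor after detonation.
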(event `self.ReceiveBeginPlay`
  (`KismetSystemLibrary.Delay` 0.2)
  (`self.Detonate`))

(event `Detonate`
  (bind _returnvalue (`self.K2_GetActorLocation`))
  (`GameplayStatics.SpawnEmitterAtLocation` null _returnvalue)
  (`GameplayStatics.ApplyRadialDamage` :`BaseDamage` (`self.GDamage`) :`Origin` _returnvalue :`DamageRadius` (`self.DamageRadius`) :`DamageCauser` self :`InstigatedByController` (`self.GetInstigatorController`))
  (`RadialForceComponent.FireImpulse` (`self.RadialForce`))
  (`GameplayStatics.PlaySoundAtLocation` "/Game/ExplosiveBarrel/ExplosionSound/ExplosionSound_Cue.ExplosionSound_Cue" _returnvalue (struct) 1.0 1.0 0.0 null null null))

(fn `UserConstructionScript`)