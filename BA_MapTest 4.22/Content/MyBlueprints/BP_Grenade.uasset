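; BP_Grenade is a timed grenade that explodes and pushes its surroundings with a radial impulse.
; On BeginPlay it waits for Duration, spawns a scaled-up particle effect at the capsule, fires the RadialForce impulse and destroys itself.
; The first Hit event zeroes the RotatingMovement rate to stop the spin, without affecting the fuse.
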(event `self.ReceiveBeginPlay`
  (bind (_returnvalue_location _returnvalue_rotation) (`KismetMathLibrary.BreakTransform` (`SceneComponent.K2_GetComponentToWorld` (`self.Capsule`))))
  (`KismetSystemLibrary.Delay` (`self.Duration`))
  (`GameplayStatics.SpawnEmitterAtLocation` null _returnvalue_location _returnvalue_rotation (6.0 6.0 6.0))
  (`RadialForceComponent.FireImpulse` (`self.RadialForce`))
  (`self.K2_DestroyActor`))

(event `self.ReceiveHit`
  (params (MyComp :type "PrimitiveComponent Object Reference") (Other :type "Actor Object Reference") (OtherComp :type "PrimitiveComponent Object Reference") (bSelfMoved :type Boolean) (HitLocation :type "Vector Structure") (HitNormal :type "Vector Structure") (NormalImpulse :type "Vector Structure") (Hit :type "HitResult Structure (by ref)"))
  (`/Engine/EditorBlueprintResources/StandardMacros.DoOnce` false
    (:`Completed`
      (set `RotatingMovementComponent.RotationRate` (struct) (`self.RotatingMovement`)))))

(fn `UserConstructionScript`)