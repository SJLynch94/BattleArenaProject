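; Grenade ammo box that holds a limited stock and refills the first-person character's ammo through a Take event.
; Take lowers Left, clamped between zero and Total, and passes the full requested Amount to AddAmmo unless the box is empty.
; Every Tick pushes Left and Total into a Widget_Amount display and turns it toward the player.
; The construction script sizes the sphere trigger from TriggerRadius.
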(event `Set Amount`
  ;[1 1 1] Setting the Widget Amount
  (bind _aswidget_amount (cast `/Game/Project/Widgets/Widget_Amount` (`WidgetComponent.GetUserWidgetObject` (`self.Widget`))))
  (set `/Game/Project/Widgets/Widget_Amount.Left` (`self.Left`) _aswidget_amount)
  (set `/Game/Project/Widgets/Widget_Amount.Total` (`self.Total`) _aswidget_amount))

(event `Rotate Widget`
  (bind _widget (`self.Widget`))
  ;[1 1 1] Rotate Widget
  (`SceneComponent.K2_SetWorldRotation` _widget (`KismetMathLibrary.FindLookAtRotation` (`SceneComponent.K2_GetComponentLocation` _widget) (`self.K2_GetActorLocation` (`GameplayStatics.GetPlayerCharacter` 0))) false false))

(event `self.ReceiveTick`
  (params (DeltaSeconds :type "Float (single-precision)"))
  (`|ExecutionSequence`
    (:`then_0`
      (`self.Set Amount`))
    (:`then_1`
      (`self.Rotate Widget`))))

(event `Take`
  (params (Amount :type Integer))
  ;[1 1 1] Taking Ammo From Box And Adding Same Value to FPC Ammo
  ;;[1 1 1] Checks if There is no more Ammo Left In Box
  (if (not (== (`self.Left`) 0))
    (set `self.Left` (`KismetMathLibrary.Clamp` (- (`self.Left`) Amount) 0 (`self.Total`)))
    ;;[1 1 1] Cast to FPC and Adding Ammo
    (bind _asfirst_person_character (cast `/Game/Project/Blueprints/FirstPersonCharacter` (`GameplayStatics.GetPlayerPawn` 0)))
    (`/Game/Project/Blueprints/FirstPersonCharacter.Add Ammo` _asfirst_person_character Amount)))

(fn `UserConstructionScript`
  (`SphereComponent.SetSphereRadius` (`self.Trigger`) (`self.Trigger Radius`) true))