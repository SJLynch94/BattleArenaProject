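; Game mode that handles respawns, kill scoring and a match countdown.
; BeginPlay runs an EQS query to spawn the first AI and binds the kill event, which respawns dead players immediately and dead AI after a delay.
; Non-player kills award points to the killer's PlayerState.
; EQS callbacks spawn pawns with debug spheres and prints, and a delay-throttled Tick counts down minutes and seconds, then calls the player pawn's PauseGame.
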(event `OnQueryPlayerSpawnFinishedEvent`
  (params (QueryInstance :type "EnvQueryInstanceBlueprintWrapper Object Reference") (QueryStatus :type "EEnvQueryStatus Enum" :default "Processing"))
  (bind _returnvalue (`GameplayStatics.GetPlayerPawn` 0))
  (switch `EEnvQueryStatus` QueryStatus
    (:`Success`
      (for _array_element (`EnvQueryInstanceBlueprintWrapper.GetResultsAsLocations` QueryInstance)
        _)
      (`KismetSystemLibrary.DrawDebugSphere` _array_element 50.0 12 (struct :`G` 0.982744 :`B` 1.0 :`A` 1.0) 2.0 2.0)
      (`self.RestartPlayer` (`Pawn.GetController` _returnvalue))
      (bind _returnvalue_2 (`|SpawnActorFromClass` "/Game/MyBlueprints/BP_PlayerPawnTest.BP_PlayerPawnTest_C" (`KismetMathLibrary.MakeTransform` _array_element) "AdjustIfPossibleButDontSpawnIfColliding" "OverrideRootScale" null null _returnvalue))
      (`KismetSystemLibrary.PrintString` (`KismetSystemLibrary.GetDisplayName` _returnvalue_2)))))

(event `OnActorKilledEvent` :!signature `self.OnActorKilled`
  (params (VictimActor :type "Actor Object Reference") (KillerActor :type "Actor Object Reference") (KillerController :type "Controller Object Reference"))
  (bind _aspawn (cast `Pawn` VictimActor))
  (if (`Pawn.IsPlayerControlled` _aspawn)
    (bind _asbp_player_pawn_test (cast `/Game/MyBlueprints/BP_PlayerPawnTest` VictimActor))
    (if (`HeroCharacter.bDied` _asbp_player_pawn_test)
      (bind _returnvalue (`EnvQueryManager.RunEQSQuery` "/Game/GameMode/EQSFindSpawnPoint/EQS_FindPlayerSpawnPoint.EQS_FindPlayerSpawnPoint" _asbp_player_pawn_test "RandomBest25Pct"))
      (add `EnvQueryInstanceBlueprintWrapper.OnQueryFinishedEvent` _returnvalue (delegate `OnQueryPlayerSpawnFinishedEvent`)))
    (else
      (bind _asbaplayer_state (cast `BAPlayerState` (`Pawn.PlayerState` (`Controller.K2_GetPawn` KillerController))))
      (`BAPlayerState.AddScore` _asbaplayer_state 10.0)
      (bind _asbp_advance_ai (cast `/Game/AdvanceAI/BP_AdvanceAI` VictimActor))
      (if (`HeroCharacter.bDied` _asbp_advance_ai)
        (`KismetSystemLibrary.Delay` 3.0)
        (bind _returnvalue_2 (`EnvQueryManager.RunEQSQuery` "/Game/GameMode/EQSFindSpawnPoint/EQS_FindAISpawnPoint.EQS_FindAISpawnPoint" self "RandomBest25Pct" :!label _label))
        (add `EnvQueryInstanceBlueprintWrapper.OnQueryFinishedEvent` _returnvalue_2 (delegate `OnQueryAISpawnFinishedEvent`))
        (add `self.OnActorKilled` (delegate `OnActorKilledEvent`))))))

(event `self.ReceiveBeginPlay`
  (goto _label))

(event `OnQueryAISpawnFinishedEvent`
  (params (QueryInstance :type "EnvQueryInstanceBlueprintWrapper Object Reference") (QueryStatus :type "EEnvQueryStatus Enum" :default "Processing"))
  (switch `EEnvQueryStatus` QueryStatus
    (:`Success`
      (for _array_element (`EnvQueryInstanceBlueprintWrapper.GetResultsAsLocations` QueryInstance)
        _)
      (`KismetSystemLibrary.DrawDebugSphere` _array_element 50.0 12 (struct :`G` 0.982744 :`B` 1.0 :`A` 1.0) 2.0 2.0)
      (bind _returnvalue (`|SpawnActorFromClass` "/Game/AdvanceAI/BP_AdvanceAI.BP_AdvanceAI_C" (`KismetMathLibrary.MakeTransform` _array_element) "AdjustIfPossibleButDontSpawnIfColliding" "OverrideRootScale" null null))
      (`KismetSystemLibrary.PrintString` (`KismetSystemLibrary.GetDisplayName` _returnvalue)))))

(event `self.ReceiveTick`
  (params (DeltaSeconds :type "Float (single-precision)"))
  (`KismetSystemLibrary.Delay` 1.0)
  (set `self.Seconds` (- (`self.Seconds`) 1))
  (if (< (`self.Seconds`) 0)
    (set `self.Seconds` 59)
    (set `self.Minutes` (- (`self.Minutes`) 1))
    (if (<= (`self.Minutes`) -1)
      (bind _asbp_player_pawn_test (cast `/Game/MyBlueprints/BP_PlayerPawnTest` (`GameplayStatics.GetPlayerPawn` 0)))
      (`/Game/MyBlueprints/BP_PlayerPawnTest.PauseGame` _asbp_player_pawn_test)
      (elif true
        _))))

(fn `UserConstructionScript`)