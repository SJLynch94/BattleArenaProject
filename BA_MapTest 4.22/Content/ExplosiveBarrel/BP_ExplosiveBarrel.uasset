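; Explosive barrel actor Blueprint that drives a floating health bar for the barrel.
; Each Tick it sets the widget's progress bar from the HealthComp's current-to-default health ratio and rotates the widget component to face the player character.
; The bar is hidden once health reaches zero.
; This graph contains no damage or explosion logic.
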(event `self.ReceiveTick`
  (params (DeltaSeconds :type "Float (single-precision)"))
  (bind _healthcomp (`self.HealthComp`))
  (bind _explosivebarrelhealthbar (`self.ExplosiveBarrelHealthBar`))
  (bind _aswbp_explosive_barrel_health_bar (cast `/Game/MyHUD/WBP_ExplosiveBarrelHealthBar` (`WidgetComponent.GetUserWidgetObject` (`self.ExplosiveBarrelHealthBar`))))
  (`ProgressBar.SetPercent` (`/Game/MyHUD/WBP_ExplosiveBarrelHealthBar.ExplosiveHealthBar` _aswbp_explosive_barrel_health_bar) (/ (`HealthComponent.Health` _healthcomp) (`HealthComponent.DefaultHealth` _healthcomp)))
  (`SceneComponent.K2_SetWorldRotation` _explosivebarrelhealthbar (`KismetMathLibrary.FindLookAtRotation` (`SceneComponent.K2_GetComponentLocation` _explosivebarrelhealthbar) (`self.K2_GetActorLocation` (`GameplayStatics.GetPlayerCharacter` 0))) false false)
  (if (<= (`HealthComponent.Health` (`self.HealthComp`)) 0.0)
    (`SceneComponent.SetVisibility` (`self.ExplosiveBarrelHealthBar`) false false)))

(fn `UserConstructionScript`)