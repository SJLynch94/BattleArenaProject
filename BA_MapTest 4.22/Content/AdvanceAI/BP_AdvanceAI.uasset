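; BP_AdvanceAI is an AI actor that runs the BT_AdvanceAI behavior tree on BeginPlay and reports damage and death through UI.
; Health component changes show debug and HUD damage text and add a hitmarker widget.
; Tick updates the world-space health bar and rotates it toward the player.
; While health is zero or below, Tick hides the bar and adds a new kill-feed popup every frame, with no once-only guard.
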(event `self.ReceiveBeginPlay`
  (`AIController.RunBehaviorTree` (`AIBlueprintHelperLibrary.GetAIController` self) "/Game/AdvanceAI/BT_AdvanceAI.BT_AdvanceAI"))

(event `self.HealthComp.OnHealthChanged`
  (params (HealthComp :type "HealthComponent Object Reference") (Health :type "Float (single-precision)") (HealthDelta :type "Float (single-precision)") (DamageType :type "DamageType Object Reference") (InstigatedBy :type "Controller Object Reference") (DamageCauser :type "Actor Object Reference"))
  (bind _returnvalue (`KismetTextLibrary.Conv_DoubleToText` HealthDelta "HalfToEven" true 1 324 0 0))
  (bind _returnvalue_2 (`self.K2_GetActorLocation`))
  (`KismetSystemLibrary.DrawDebugString` _returnvalue_2 (`KismetTextLibrary.Conv_TextToString` _returnvalue) null (struct :`R` 1.0 :`G` 0.651406 :`A` 1.0) 0.75)
  (message `/Game/UI/ShowDamageText.ShowDamageText` (`PlayerController.GetHUD` (`GameplayStatics.GetPlayerController` 0)) true (`KismetTextLibrary.Conv_TextToString` _returnvalue) _returnvalue_2)
  (bind _returnvalue_3 (`|CreateWidget` "/Game/MyHUD/WBP_Hitmarker.WBP_Hitmarker_C"))
  (`UserWidget.AddToViewport` _returnvalue_3 0))

(event `self.ReceiveTick`
  (params (DeltaSeconds :type "Float (single-precision)"))
  (bind _healthcomp (`self.HealthComp`))
  (bind _aihealthbar (`self.AIHealthBar`))
  (bind _aswbp_aihealth_bar (cast `/Game/MyHUD/WBP_AIHealthBar` (`WidgetComponent.GetUserWidgetObject` (`self.AIHealthBar`))))
  (`ProgressBar.SetPercent` (`/Game/MyHUD/WBP_AIHealthBar.AIHealthBar` _aswbp_aihealth_bar) (/ (`HealthComponent.Health` _healthcomp) (`HealthComponent.DefaultHealth` _healthcomp)))
  (`SceneComponent.K2_SetWorldRotation` _aihealthbar (`KismetMathLibrary.FindLookAtRotation` (`SceneComponent.K2_GetComponentLocation` _aihealthbar) (`self.K2_GetActorLocation` (`GameplayStatics.GetPlayerCharacter` 0))) false false)
  (if (<= (`HealthComponent.Health` (`self.HealthComp`)) 0.0)
    (`SceneComponent.SetVisibility` (`self.AIHealthBar`) false false)
    (bind _returnvalue (`|CreateWidget` "/Game/MyHUD/WBP_KillFeedPopup.WBP_KillFeedPopup_C"))
    (`UserWidget.AddToViewport` _returnvalue 0)))

(fn `UserConstructionScript`)