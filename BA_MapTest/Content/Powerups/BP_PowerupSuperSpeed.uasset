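; Super speed powerup that temporarily doubles the walk speed of the actor it is activated for.
; On activation it stores that actor and sets MaxWalkSpeed to twice the movement component's current GetMaxSpeed.
; On expiry it halves the current max speed instead of restoring a saved value, if the actor is still valid.
; It also plays a powerdown cue at player 0's location, then calls the parent's expiry logic.
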(event `self.OnActivated`
  (params (ActivateFor :type "Actor Object Reference"))
  (bind _returnvalue (`self.GetComponentByClass` ActivateFor "/Script/Engine.CharacterMovementComponent"))
  (set `self.ActivatedFor` ActivateFor)
  (set `CharacterMovementComponent.MaxWalkSpeed` (* (`MovementComponent.GetMaxSpeed` _returnvalue) 2.0) _returnvalue))

(event `self.OnExpired`
  (bind _activatedfor (`self.ActivatedFor`))
  (bind _returnvalue (`self.GetComponentByClass` _activatedfor "/Script/Engine.CharacterMovementComponent"))
  (`/Engine/EditorBlueprintResources/StandardMacros.IsValid` _activatedfor
    (:`Is Valid`
      (set `CharacterMovementComponent.MaxWalkSpeed` (/ (`MovementComponent.GetMaxSpeed` _returnvalue) 2.0) _returnvalue)
      (`GameplayStatics.PlaySoundAtLocation` "/Game/Powerups/powerdown_01_Cue.powerdown_01_Cue" (`self.K2_GetActorLocation` (`GameplayStatics.GetPlayerPawn` 0))))
    (:`Is Not Valid`
      _))
  (`parent.OnExpired`))

(fn `UserConstructionScript`)